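; Beast actor for the labyrinth that appears, travels between two path nodes, then removes itself.
; On BeginPlay, the Reveal timeline animates the mesh from a lowered offset before movement begins at StartNode.
; Tick steps through the player character's NodeLocations toward EndNode in either index direction, moving at constant BeastSpeed and facing each next node.
; At EndNode, Tick calls Despawn, which reverse-plays a second timeline on the mesh and destroys the actor when finished.
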(event `self.ReceiveBeginPlay`
  (`SceneComponent.K2_SetRelativeLocation` (`self.StaticMesh`) (0.0 0.0 -180.0) false false)
  (bind (_direction _location) (`Timeline|Reveal` :!via `PlayFromStart`)
    (:`Update`
      (`SceneComponent.K2_SetRelativeLocation` (`self.StaticMesh`) _location false false))
    (:`Finished`
      (set `self.HasSpawned` true)
      (set `self.CurrentNode` (`self.StartNode`)))))

(event `Despawn`
  (bind (_direction _location) (`Timeline|Timeline_0` :!via `ReverseFromEnd`)
    (:`Update`
      (`SceneComponent.K2_SetRelativeLocation` (`self.StaticMesh`) _location false false))
    (:`Finished`
      (`self.K2_DestroyActor`))))

(event `self.ReceiveTick`
  (params (DeltaSeconds :type "Float (single-precision)"))
  (bind _defaultsceneroot (`self.DefaultSceneRoot`))
  (bind _beastspeed (`self.BeastSpeed`))
  (bind _currentnode (`self.CurrentNode`))
  (bind _endnode (`self.EndNode`))
  (bind _currentnode_2 (`self.CurrentNode`))
  (bind _currentnode_3 (`self.CurrentNode`))
  (bind _returnvalue (`SceneComponent.K2_GetComponentLocation` (`self.DefaultSceneRoot`)))
  (bind _nodelocations (`/Game/Blueprint/Gameplay/BP_Character_Labyrinth.NodeLocations` (cast `/Game/Blueprint/Gameplay/BP_Character_Labyrinth` (`GameplayStatics.GetPlayerCharacter` 0) :!pure true)))
  (bind _output (`|GetArrayItem` _nodelocations (+ _currentnode_2 1)))
  (bind _output_2 (`|GetArrayItem` _nodelocations (- _currentnode_2 1)))
  (if (`self.HasSpawned`)
    (if (== _currentnode_3 _endnode)
      (set `self.IsDespawning` true)
      (`self.Despawn`)
      (elif (> _currentnode_3 _endnode)
        (`SceneComponent.K2_SetWorldLocationAndRotation` _defaultsceneroot (`KismetMathLibrary.VInterpTo_Constant` _returnvalue _output_2 DeltaSeconds _beastspeed) (`KismetMathLibrary.FindLookAtRotation` _returnvalue _output_2) false false)
        (if (== _returnvalue _output_2 :`ErrorTolerance` 0.1)
          (set `self.CurrentNode` (- _currentnode 1)))
        (elif (< _currentnode_3 _endnode)
          (`SceneComponent.K2_SetWorldLocationAndRotation` _defaultsceneroot (`KismetMathLibrary.VInterpTo_Constant` _returnvalue _output DeltaSeconds _beastspeed) (`KismetMathLibrary.FindLookAtRotation` _returnvalue _output) false false)
          (if (== _returnvalue _output :`ErrorTolerance` 0.1)
            (set `self.CurrentNode` (+ _currentnode 1))))))))

(fn `UserConstructionScript`)