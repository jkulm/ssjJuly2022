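; BP_Character is a character Blueprint that exposes animation blend controls for selectable characters such as Drummo and Noodler.
; SetAnimSlotBlend and SetHeadSlotBlend branch on CharacterSelection, cast the skeletal mesh's anim instance to that character's AnimBP, and write BlendSequence or BlendDisapprove respectively.
; A third selection is stubbed with no effect, and the event graph and construction script are empty.
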(event `self.ReceiveTick`
  (params (DeltaSeconds :type "Float (single-precision)")))

(fn `SetAnimSlotBlend`
  (params (Blend :type "Float (double-precision)"))
  (bind _characterselection (`self.CharacterSelection`))
  (bind _returnvalue (`SkeletalMeshComponent.GetAnimInstance` (`self.SkeletalMesh`)))
  (if (== _characterselection 0)
    (bind _asabp_drummo (cast `/Game/Art/Character/Drummo/Animation/ABP_Drummo` _returnvalue))
    (set `/Game/Art/Character/Drummo/Animation/ABP_Drummo.BlendSequence` Blend _asabp_drummo)
    (elif (== _characterselection 1)
      (bind _asabp_noodler (cast `/Game/Art/Character/Noodler/ABP_Noodler` _returnvalue))
      (set `/Game/Art/Character/Noodler/ABP_Noodler.BlendSequence` Blend _asabp_noodler)
      (elif (== _characterselection 2)
        _))))

(fn `SetHeadSlotBlend`
  (params (Blend :type "Float (double-precision)"))
  (bind _characterselection (`self.CharacterSelection`))
  (bind _returnvalue (`SkeletalMeshComponent.GetAnimInstance` (`self.SkeletalMesh`)))
  (if (== _characterselection 0)
    (bind _asabp_drummo (cast `/Game/Art/Character/Drummo/Animation/ABP_Drummo` _returnvalue))
    (set `/Game/Art/Character/Drummo/Animation/ABP_Drummo.BlendDisapprove` Blend _asabp_drummo)
    (elif (== _characterselection 1)
      (bind _asabp_noodler (cast `/Game/Art/Character/Noodler/ABP_Noodler` _returnvalue))
      (set `/Game/Art/Character/Noodler/ABP_Noodler.BlendDisapprove` Blend _asabp_noodler)
      (elif (== _characterselection 2)
        _))))

(fn `UserConstructionScript`)