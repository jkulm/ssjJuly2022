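; BP_Drum is a grabbable puzzle drum that plays its selected note when grabbed and reports it to BP_PuzzleManager, which it looks up on BeginPlay.
; The construction script sets the note's audio event and reverb and creates a dynamic drumhead material.
; Each hit starts a drumhead animation value that decays on Tick.
; Separate events set the head color and configure or trigger a Niagara ring effect.
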(event `self.ReceiveBeginPlay`
  (bind _outactors (`GameplayStatics.GetAllActorsOfClass` "/Game/Blueprint/PuzzleManagers/BP_PuzzleManager.BP_PuzzleManager_C" :!label _label))
  (bind _output (`|GetArrayItem` _outactors))
  (`/Engine/EditorBlueprintResources/StandardMacros.IsValid` _output
    (:`Is Valid`
      (set `self.PuzzleManagerRef` _output))
    (:`Is Not Valid`
      (goto _label))))

(event `self.ReceiveTick`
  (params (DeltaSeconds :type "Float (single-precision)"))
  (bind _drumanimation (`self.DrumAnimation`))
  (if (> _drumanimation 0.0)
    (bind _output_get (set `self.DrumAnimation` (- _drumanimation (/ 1.0 (`self.DrumHeadDecay`)))))
    (`MaterialInstanceDynamic.SetScalarParameterValue` (`self.DrumHeadMat`) "BP_Value" _output_get)))

(event `/Game/Blueprint/Interfaces/BPI_Grab.GrabObject`
  (params (HitCollider :type "PrimitiveComponent Object Reference"))
  (`FMODBlueprintStatics.PlayEventAtLocation` (`|GetArrayItem` (`self.NoteList`) (`self.NoteSelection`)) (`KismetMathLibrary.MakeTransform` (`SceneComponent.K2_GetComponentLocation` (`self.Notes`))))
  (set `self.DrumAnimation` 1.0)
  (`/Game/Blueprint/PuzzleManagers/BP_PuzzleManager.PlayerInput` (`self.PuzzleManagerRef`) (`self.NoteSelection`) self))

(event `/Game/Blueprint/Interfaces/BPI_Grab.ReleaseObject`)

(event `Set Color`
  (params (Color :type "LinearColor Structure"))
  (`MaterialInstanceDynamic.SetVectorParameterValue` (`self.DrumHeadMat`) "BP_Color" Color))

(event `TriggerRing`
  (`ActorComponent.Activate` (`self.Niagara`) true))

(event `SetRingDefaults`
  (params (Duration :type "Float (double-precision)"))
  (`FXSystemComponent.SetFloatParameter` (`self.Niagara`) "User.Duration" Duration))

(fn `UserConstructionScript`
  (bind _mesh (`self.Mesh`))
  (`FMODAudioComponent.SetEvent` (`self.Notes`) (`|GetArrayItem` (`self.NoteList`) (`self.NoteSelection`)))
  (`FMODAudioComponent.SetParameter` (`self.Notes`) "Reverb" (`self.Reverb`))
  (bind _returnvalue (`PrimitiveComponent.CreateDynamicMaterialInstance` _mesh 2 (`PrimitiveComponent.GetMaterial` _mesh 2) "None"))
  (set `self.DrumHeadMat` _returnvalue))