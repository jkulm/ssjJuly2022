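; Grabbable bass actor with five strings that each play a note and animate when grabbed.
; GrabObject matches the hit collider to a string, plays that string's note from NoteList and sets its animation value to full.
; Tick lowers each value by a fixed, frame-rate-dependent step and feeds it to the dynamic string material.
; The construction script builds the material and collider list, and applies Reverb to the first note only.
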(event `self.ReceiveTick`
  (params (DeltaSeconds :type "Float (single-precision)"))
  (bind _stringanimdecay (`self.StringAnimDecay`))
  ;[1 1 1] Decay Animation Values
  (`|ExecutionSequence`
    (:`then_0`
      (bind _outvalue (`self.AnimDecay` (`self.String1Animation`) _stringanimdecay))
      (bind _output_get (set `self.String1Animation` _outvalue))
      (`MaterialInstanceDynamic.SetScalarParameterValue` (`self.StringMat`) "BP_Value1" _output_get))
    (:`then_1`
      (bind _outvalue_2 (`self.AnimDecay` (`self.String2Animation`) _stringanimdecay))
      (bind _output_get_2 (set `self.String2Animation` _outvalue_2))
      (`MaterialInstanceDynamic.SetScalarParameterValue` (`self.StringMat`) "BP_Value2" _output_get_2))
    (:`then_2`
      (bind _outvalue_3 (`self.AnimDecay` (`self.String3Animation`) _stringanimdecay))
      (bind _output_get_3 (set `self.String3Animation` _outvalue_3))
      (`MaterialInstanceDynamic.SetScalarParameterValue` (`self.StringMat`) "BP_Value3" _output_get_3))
    (:`then_3`
      (bind _outvalue_4 (`self.AnimDecay` (`self.String4Animation`) _stringanimdecay))
      (bind _output_get_4 (set `self.String4Animation` _outvalue_4))
      (`MaterialInstanceDynamic.SetScalarParameterValue` (`self.StringMat`) "BP_Value4" _output_get_4))
    (:`then_4`
      (bind _outvalue_5 (`self.AnimDecay` (`self.String5Animation`) _stringanimdecay))
      (bind _output_get_5 (set `self.String5Animation` _outvalue_5))
      (`MaterialInstanceDynamic.SetScalarParameterValue` (`self.StringMat`) "BP_Value5" _output_get_5))))

(event `/Game/Blueprint/Interfaces/BPI_Grab.GrabObject`
  (params (HitCollider :type "PrimitiveComponent Object Reference"))
  (bind _stringcolliders (`self.StringColliders`))
  (bind _note1 (`self.Note1`))
  (bind _note2 (`self.Note2`))
  (bind _note3 (`self.Note3`))
  (bind _note4 (`self.Note4`))
  (bind _note5 (`self.Note5`))
  (bind _returnvalue (`KismetArrayLibrary.Array_Find` _stringcolliders HitCollider))
  (bind _output (`|GetArrayItem` (`self.NoteList`) _returnvalue))
  (if (`KismetArrayLibrary.Array_Contains` _stringcolliders HitCollider)
    (`|ExecutionSequence`
      (:`then_0`
        (if (== _returnvalue 0)
          (set `self.String1Animation` 1.0)
          (`FMODAudioComponent.SetEvent` _note1 _output)
          (`FMODAudioComponent.Play` _note1)))
      (:`then_1`
        (if (== _returnvalue 1)
          (set `self.String2Animation` 1.0)
          (`FMODAudioComponent.SetEvent` _note2 _output)
          (`FMODAudioComponent.Play` _note2)))
      (:`then_2`
        (if (== _returnvalue 2)
          (set `self.String3Animation` 1.0)
          (`FMODAudioComponent.SetEvent` _note3 _output)
          (`FMODAudioComponent.Play` _note3)))
      (:`then_3`
        (if (== _returnvalue 3)
          (set `self.String4Animation` 1.0)
          (`FMODAudioComponent.SetEvent` _note4 _output)
          (`FMODAudioComponent.Play` _note4)))
      (:`then_4`
        (if (== _returnvalue 4)
          (set `self.String5Animation` 1.0)
          (`FMODAudioComponent.SetEvent` _note5 _output)
          (`FMODAudioComponent.Play` _note5))))))

(event `/Game/Blueprint/Interfaces/BPI_Grab.ReleaseObject`)

(fn `AnimDecay`
  (params (InValue :type "Float (double-precision)") (DecayRate :type "Float (double-precision)"))
  (returns (OutValue :type "Float (double-precision)"))
  (if (> InValue 0.0)
    (return (- InValue (/ 1.0 DecayRate)))))

(fn `UserConstructionScript`
  (bind _mesh (`self.Mesh`))
  (bind _stringcolliders (`self.StringColliders`))
  (`FMODAudioComponent.SetEvent` (`self.Note1`) (`|GetArrayItem` (`self.NoteList`) (`self.NoteSelection`)))
  (`FMODAudioComponent.SetParameter` (`self.Note1`) "Reverb" (`self.Reverb`))
  (bind _returnvalue (`PrimitiveComponent.CreateDynamicMaterialInstance` _mesh 2 (`PrimitiveComponent.GetMaterial` _mesh 2) "None"))
  (set `self.StringMat` _returnvalue)
  (`KismetArrayLibrary.Array_Clear` _stringcolliders)
  (`KismetArrayLibrary.Array_Add` _stringcolliders (`self.String1`))
  (`KismetArrayLibrary.Array_Add` _stringcolliders (`self.String2`))
  (`KismetArrayLibrary.Array_Add` _stringcolliders (`self.String3`))
  (`KismetArrayLibrary.Array_Add` _stringcolliders (`self.String4`))
  (`KismetArrayLibrary.Array_Add` _stringcolliders (`self.String5`)))