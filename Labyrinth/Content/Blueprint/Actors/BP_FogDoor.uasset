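; BP_FogDoor is a fog barrier actor that can be switched on and off, with a Niagara effect and an eroding plane material.
; SetActiveState enables collision and plays a timeline forward, or reverses it and disables actor collision when it finishes.
; The timeline drives the Niagara fade and the dynamic material's Erosion parameter together.
; The construction script creates that material and sets the initial visuals, collision and state from OverrideActive.
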(event `SetActiveState`
  (params (State :type Boolean))
  (bind _material (`self.Material`))
  (bind _niagara (`self.Niagara`))
  (bind _output_get (set `self.State` State))
  (`ActorComponent.SetActive` (`self.BoxCollider`) _output_get false)
  (if _output_get
    (`ActorComponent.Activate` _niagara true)
    (`self.SetActorEnableCollision` true)
    (bind (_direction _time) (`Timeline|TimeTimeline` :`NewTime` 4.0 :!label _label)
      (:`Update`
        (bind _output_get_2 (set `self.Time` _time))
        (if _output_get
          (`FXSystemComponent.SetFloatParameter` _niagara "User.Fade" _output_get_2)
          (`MaterialInstanceDynamic.SetScalarParameterValue` _material "Erosion" _output_get_2)
          (else
            (`FXSystemComponent.SetFloatParameter` _niagara "User.Fade" _output_get_2)
            (`MaterialInstanceDynamic.SetScalarParameterValue` _material "Erosion" _output_get_2))))
      (:`Finished`
        (if (not _output_get)
          (`ActorComponent.Activate` _niagara false)
          (`self.SetActorEnableCollision` false))))
    (else
      (goto _label :!via `Reverse`))))

(fn `UserConstructionScript`
  (bind _plane (`self.Plane`))
  (bind _material (`self.Material`))
  (bind _niagara (`self.Niagara`))
  (bind _returnvalue (`PrimitiveComponent.CreateDynamicMaterialInstance` _plane 0 (`PrimitiveComponent.GetMaterial` _plane 0) "None"))
  (set `self.Material` _returnvalue)
  (if (`self.OverrideActive`)
    (`MaterialInstanceDynamic.SetScalarParameterValue` _material "Erosion" 1.0)
    (`ActorComponent.SetAutoActivate` _niagara true)
    (`self.SetActorEnableCollision` true)
    (set `self.State` true)
    (else
      (`MaterialInstanceDynamic.SetScalarParameterValue` _material "Erosion" 0.0)
      (`ActorComponent.SetAutoActivate` _niagara false)
      (`self.SetActorEnableCollision` false)
      (set `self.State` false))))