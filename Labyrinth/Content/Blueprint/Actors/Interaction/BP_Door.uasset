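; BP_Door is an interactable door actor that toggles between open and closed on each Interact call.
; The TL_OpenDoor timeline plays or reverses to lerp the Door component's relative yaw between zero and a quarter turn either way.
; With AlwaysOpenAway set, opening first dots the player-to-door direction with the actor's forward vector, and the sign picks the swing side so it opens away from the player.
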(event `self.ReceiveBeginPlay`
  (`parent.ReceiveBeginPlay`))

(event `/Game/Blueprint/Interfaces/BPI_Interaction.Interact`
  (if (`self.IsDoorClosed`)
    (set `self.IsDoorClosed` false)
    (if (`self.AlwaysOpenAway`)
      (set `self.PlayerDotProduct` (`KismetMathLibrary.Dot_VectorVector` (`KismetMathLibrary.Normal` (- (`self.K2_GetActorLocation` self) (`self.K2_GetActorLocation` (`self.PlayerRef`)))) (`self.GetActorForwardVector` self)))
      (bind (_direction _alpha) (`Timeline|TL_OpenDoor` :!label _label)
        (:`Update`
          (`SceneComponent.K2_SetRelativeRotation` (`self.Door`) (`KismetMathLibrary.MakeRotator` 0.0 0.0 (`KismetMathLibrary.Lerp` 0.0 (* (select `bool` (>= (`self.PlayerDotProduct`) 0.0) :`false` 1.0 :`true` -1.0 :!type "Float (single-precision)") -90.0) _alpha)) false false)))
      (else
        (goto _label)))
    (else
      (set `self.IsDoorClosed` true)
      (goto _label :!via `Reverse`))))

(fn `UserConstructionScript`
  (`parent.UserConstructionScript`))