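; Base actor for readable notes that glow near the Labyrinth player and open an examination widget when the Action input is pressed.
; While the player overlaps the sphere, Tick traces to the camera, lighting a dynamic paper material when unobstructed and enabling input only within pickup distance.
; The widget receives the note and the level's BP_NoteExamination actor.
; The construction script applies the note text and sphere radius.
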(event `self.ReceiveBeginPlay`
  (bind _returnvalue (`GameplayStatics.GetActorOfClass` "/Game/Blueprint/Actors/Notes/BP_NoteExamination.BP_NoteExamination_C"))
  (set `self.NoteExaminationRef` _returnvalue))

(event `self.OverlapSphere.OnComponentBeginOverlap`
  (params (OverlappedComponent :type "PrimitiveComponent Object Reference") (OtherActor :type "Actor Object Reference") (OtherComp :type "PrimitiveComponent Object Reference") (OtherBodyIndex :type Integer) (bFromSweep :type Boolean) (SweepResult :type "HitResult Structure (by ref)"))
  (bind _asbp_character_labyrinth (cast `/Game/Blueprint/Gameplay/BP_Character_Labyrinth` OtherActor))
  (set `self.PlayerRef` _asbp_character_labyrinth)
  (`MaterialInstanceDynamic.SetVectorParameterValue` (`self.NoteMaterial`) "Glow" (`self.GlowColor`))
  (set `self.UpdateActor` true))

(event `self.OverlapSphere.OnComponentEndOverlap`
  (params (OverlappedComponent :type "PrimitiveComponent Object Reference") (OtherActor :type "Actor Object Reference") (OtherComp :type "PrimitiveComponent Object Reference") (OtherBodyIndex :type Integer))
  (cast `/Game/Blueprint/Gameplay/BP_Character_Labyrinth` OtherActor)
  (set `self.UpdateActor` false)
  (`MaterialInstanceDynamic.SetVectorParameterValue` :`self` (`self.NoteMaterial`) :`ParameterName` "Glow")
  (`self.DisableInput` (`GameplayStatics.GetPlayerController` 0)))

(event `self.ReceiveTick`
  (params (DeltaSeconds :type "Float (single-precision)"))
  (bind _returnvalue (`GameplayStatics.GetPlayerController` 0))
  (bind _notematerial (`self.NoteMaterial`))
  (if (`self.UpdateActor`)
    (bind (_outhit _returnvalue_2) (`KismetSystemLibrary.LineTraceSingle` (`self.K2_GetActorLocation`) (`SceneComponent.K2_GetComponentLocation` (`/Game/Blueprint/Gameplay/BP_Character_Labyrinth.Camera` (`self.PlayerRef`))) "TraceTypeQuery1"))
    (if (not _returnvalue_2)
      (`MaterialInstanceDynamic.SetVectorParameterValue` _notematerial "Glow" (`self.GlowColor`))
      (bind (_bblockinghit _binitialoverlap _time _distance _location _impactpoint _normal _impactnormal _physmat _hitactor _hitcomponent _hitbonename _hititem _elementindex _faceindex _tracestart _traceend) (`GameplayStatics.BreakHitResult` _outhit))
      (if (<= (`KismetMathLibrary.VSize` (- _tracestart _traceend)) (`self.PickUpDistance`))
        (`self.EnableInput` _returnvalue)
        (else
          (`self.DisableInput` _returnvalue)))
      (else
        (`MaterialInstanceDynamic.SetVectorParameterValue` :`self` _notematerial :`ParameterName` "Glow")
        (`self.DisableInput` (`GameplayStatics.GetPlayerController` 0))))))

(event `InputAction|Action`
  (params (Key :type "Key Structure"))
  (:`Pressed`
    (`/Engine/EditorBlueprintResources/StandardMacros.IsValid` (`self.NoteWidgetRef`)
      (:`Is Not Valid`
        (bind _returnvalue (`|CreateWidget` "/Game/UI/UMG/Menus/W_NoteExamination.W_NoteExamination_C" null (`self.NoteExaminationRef`)))
        (bind _output_get (set `self.NoteWidgetRef` _returnvalue))
        (`/Game/UI/UMG/Menus/W_NoteExamination.UpdateWidget` _output_get self)
        (`UserWidget.AddToViewport` _returnvalue 0)))))

(fn `UserConstructionScript`
  (bind _papermesh (`self.PaperMesh`))
  (`TextRenderComponent.K2_SetText` (`self.NoteText`) (`self.NoteText(Text)`))
  (bind _returnvalue (`PrimitiveComponent.CreateDynamicMaterialInstance` _papermesh 0 (`PrimitiveComponent.GetMaterial` _papermesh 0) "None"))
  (set `self.NoteMaterial` _returnvalue)
  (`SphereComponent.SetSphereRadius` (`self.OverlapSphere`) (`self.OverlapRadius`) true))