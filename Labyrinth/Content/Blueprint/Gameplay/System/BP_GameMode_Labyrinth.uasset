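; Game mode for the Labyrinth level that handles saving, loading and resetting the player's progress in the current save slot.
; LoadGame copies branch, path and fog door states from BP_SaveGame onto the Labyrinth character, plus level and start location onto itself, or creates a save with a default start location.
; SaveGame writes those values back into the existing slot.
; RestartLevel only deletes the slot, without reloading the level.
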(event `self.ReceiveBeginPlay`)

(event `LoadGame`
  (bind _asbp_character_labyrinth (cast `/Game/Blueprint/Gameplay/BP_Character_Labyrinth` (`GameplayStatics.GetPlayerCharacter` 0) :!pure true))
  (bind _returnvalue (`GameplayStatics.DoesSaveGameExist` (`self.CurrentSaveSlot`)))
  (if _returnvalue
    (bind _returnvalue_2 (`GameplayStatics.LoadGameFromSlot` (`self.CurrentSaveSlot`)))
    (bind _asbp_save_game (cast `/Game/Blueprint/Gameplay/System/BP_SaveGame` _returnvalue_2))
    (set `/Game/Blueprint/Gameplay/BP_Character_Labyrinth.BranchesStarted` (`/Game/Blueprint/Gameplay/System/BP_SaveGame.BranchesStarted` _asbp_save_game) _asbp_character_labyrinth)
    (set `/Game/Blueprint/Gameplay/BP_Character_Labyrinth.BranchesFinished` (`/Game/Blueprint/Gameplay/System/BP_SaveGame.BranchesFinished` _asbp_save_game) _asbp_character_labyrinth)
    (set `/Game/Blueprint/Gameplay/BP_Character_Labyrinth.PathStarted` (`/Game/Blueprint/Gameplay/System/BP_SaveGame.PathsStarted` _asbp_save_game) _asbp_character_labyrinth)
    (set `/Game/Blueprint/Gameplay/BP_Character_Labyrinth.PathFinished` (`/Game/Blueprint/Gameplay/System/BP_SaveGame.PathsFinished` _asbp_save_game) _asbp_character_labyrinth)
    (set `self.LevelToLoad` (`/Game/Blueprint/Gameplay/System/BP_SaveGame.LevelToLoad` _asbp_save_game))
    (set `self.StartLocation` (`/Game/Blueprint/Gameplay/System/BP_SaveGame.StartLocation` _asbp_save_game))
    (set `/Game/Blueprint/Gameplay/BP_Character_Labyrinth.FogDoorStates` (`/Game/Blueprint/Gameplay/System/BP_SaveGame.FogDoorStates` _asbp_save_game) _asbp_character_labyrinth)
    (else
      ;[1 1 1] Create save file
      (bind _returnvalue_3 (`GameplayStatics.CreateSaveGameObject` "/Game/Blueprint/Gameplay/System/BP_SaveGame.BP_SaveGame_C"))
      (set `self.StartLocation` (-7000.0 0.0 225.0))
      (`GameplayStatics.SaveGameToSlot` _returnvalue_3 (`self.CurrentSaveSlot`)))))

(event `SaveGame`
  (bind _asbp_character_labyrinth (cast `/Game/Blueprint/Gameplay/BP_Character_Labyrinth` (`GameplayStatics.GetPlayerCharacter` 0) :!pure true))
  (bind _returnvalue (`GameplayStatics.LoadGameFromSlot` (`self.CurrentSaveSlot`)))
  (bind _asbp_save_game (cast `/Game/Blueprint/Gameplay/System/BP_SaveGame` _returnvalue))
  (set `/Game/Blueprint/Gameplay/System/BP_SaveGame.BranchesStarted` (`/Game/Blueprint/Gameplay/BP_Character_Labyrinth.BranchesStarted` _asbp_character_labyrinth) _asbp_save_game)
  (set `/Game/Blueprint/Gameplay/System/BP_SaveGame.BranchesFinished` (`/Game/Blueprint/Gameplay/BP_Character_Labyrinth.BranchesFinished` _asbp_character_labyrinth) _asbp_save_game)
  (set `/Game/Blueprint/Gameplay/System/BP_SaveGame.PathsStarted` (`/Game/Blueprint/Gameplay/BP_Character_Labyrinth.PathStarted` _asbp_character_labyrinth) _asbp_save_game)
  (set `/Game/Blueprint/Gameplay/System/BP_SaveGame.PathsFinished` (`/Game/Blueprint/Gameplay/BP_Character_Labyrinth.PathFinished` _asbp_character_labyrinth) _asbp_save_game)
  (set `/Game/Blueprint/Gameplay/System/BP_SaveGame.LevelToLoad` (`self.LevelToLoad`) _asbp_save_game)
  (set `/Game/Blueprint/Gameplay/System/BP_SaveGame.StartLocation` (`self.StartLocation`) _asbp_save_game)
  (set `/Game/Blueprint/Gameplay/System/BP_SaveGame.FogDoorStates` (`/Game/Blueprint/Gameplay/BP_Character_Labyrinth.FogDoorStates` _asbp_character_labyrinth) _asbp_save_game)
  (`GameplayStatics.SaveGameToSlot` _asbp_save_game (`self.CurrentSaveSlot`)))

(event `RestartLevel`
  (`GameplayStatics.DeleteGameInSlot` (`self.CurrentSaveSlot`)))

(fn `UserConstructionScript`)