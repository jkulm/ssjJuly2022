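; Game instance for the Labyrinth game that manages a three-slot save system through BP_SaveGame.
; LoadGame copies branch, path, puzzle and fog-door progress onto the player character and sets level and start location, or creates a new save starting at the intro level.
; SaveGame writes that state back with a timestamp.
; RestartLevel deletes the current slot, and CheckSaveTime caches each slot's save time.
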(event `LoadGame`
  (bind (_returnvalue_year _returnvalue_month _returnvalue_day _returnvalue_hour _returnvalue_minute) (`KismetMathLibrary.BreakDateTime` (`KismetMathLibrary.Now`)))
  (bind _asbp_character_labyrinth (cast `/Game/Blueprint/Gameplay/BP_Character_Labyrinth` (`GameplayStatics.GetPlayerCharacter` 0) :!pure true))
  (bind _output_get (set `self.CurrentSaveSlotName` (select `int` (`self.CurrentSaveSlot`) :`0` "slot1" :`1` "slot2" :`2` "slot3")))
  (bind _returnvalue (`GameplayStatics.DoesSaveGameExist` _output_get))
  (if _returnvalue
    (bind _returnvalue_2 (`GameplayStatics.LoadGameFromSlot` (`self.CurrentSaveSlotName`)))
    (bind _asbp_save_game (cast `/Game/Blueprint/Gameplay/System/BP_SaveGame` _returnvalue_2))
    (set `/Game/Blueprint/Gameplay/BP_Character_Labyrinth.BranchesStarted` (`/Game/Blueprint/Gameplay/System/BP_SaveGame.BranchesStarted` _asbp_save_game) _asbp_character_labyrinth)
    (set `/Game/Blueprint/Gameplay/BP_Character_Labyrinth.BranchesFinished` (`/Game/Blueprint/Gameplay/System/BP_SaveGame.BranchesFinished` _asbp_save_game) _asbp_character_labyrinth)
    (set `/Game/Blueprint/Gameplay/BP_Character_Labyrinth.PathStarted` (`/Game/Blueprint/Gameplay/System/BP_SaveGame.PathsStarted` _asbp_save_game) _asbp_character_labyrinth)
    (set `/Game/Blueprint/Gameplay/BP_Character_Labyrinth.PathFinished` (`/Game/Blueprint/Gameplay/System/BP_SaveGame.PathsFinished` _asbp_save_game) _asbp_character_labyrinth)
    (set `self.LevelToLoad` (`/Game/Blueprint/Gameplay/System/BP_SaveGame.LevelToLoad` _asbp_save_game))
    (set `self.StartLocation` (`/Game/Blueprint/Gameplay/System/BP_SaveGame.StartLocation` _asbp_save_game))
    (set `/Game/Blueprint/Gameplay/BP_Character_Labyrinth.FogDoorStates` (`/Game/Blueprint/Gameplay/System/BP_SaveGame.FogDoorStates` _asbp_save_game) _asbp_character_labyrinth)
    (set `/Game/Blueprint/Gameplay/BP_Character_Labyrinth.PuzzlesFinished` (`/Game/Blueprint/Gameplay/System/BP_SaveGame.PuzzlesFinished` _asbp_save_game) _asbp_character_labyrinth)
    (else
      ;[1 1 1] Create save file
      (bind _returnvalue_3 (`GameplayStatics.CreateSaveGameObject` "/Game/Blueprint/Gameplay/System/BP_SaveGame.BP_SaveGame_C"))
      (set `/Game/Blueprint/Gameplay/System/BP_SaveGame.StartLocation` (-7000.0 0.0 475.0) _returnvalue_3)
      (set `/Game/Blueprint/Gameplay/System/BP_SaveGame.SaveTime` (`KismetStringLibrary.Concat_StrStr` (`KismetStringLibrary.Conv_IntToString` _returnvalue_year) "/" (`KismetStringLibrary.Conv_IntToString` _returnvalue_month) "/" (`KismetStringLibrary.Conv_IntToString` _returnvalue_day) " " (`KismetStringLibrary.Conv_IntToString` _returnvalue_hour) ":" (`KismetStringLibrary.Conv_IntToString` _returnvalue_minute)) _returnvalue_3)
      (set `/Game/Blueprint/Gameplay/System/BP_SaveGame.FogDoorStates` (`/Game/Blueprint/Gameplay/BP_Character_Labyrinth.FogDoorStates` (cast `/Game/Blueprint/Gameplay/BP_Character_Labyrinth` (`GameplayStatics.GetPlayerCharacter` 0) :!pure true)) _returnvalue_3)
      (set `self.LevelToLoad` "S01_Intro")
      (`GameplayStatics.SaveGameToSlot` _returnvalue_3 (`self.CurrentSaveSlotName`)))))

(event `SaveGame`
  (bind (_returnvalue_year _returnvalue_month _returnvalue_day _returnvalue_hour _returnvalue_minute) (`KismetMathLibrary.BreakDateTime` (`KismetMathLibrary.Now`)))
  (bind _asbp_character_labyrinth (cast `/Game/Blueprint/Gameplay/BP_Character_Labyrinth` (`GameplayStatics.GetPlayerCharacter` 0) :!pure true))
  (bind _returnvalue (`GameplayStatics.LoadGameFromSlot` (`self.CurrentSaveSlotName`)))
  (bind _asbp_save_game (cast `/Game/Blueprint/Gameplay/System/BP_SaveGame` _returnvalue))
  (set `/Game/Blueprint/Gameplay/System/BP_SaveGame.BranchesStarted` (`/Game/Blueprint/Gameplay/BP_Character_Labyrinth.BranchesStarted` _asbp_character_labyrinth) _asbp_save_game)
  (set `/Game/Blueprint/Gameplay/System/BP_SaveGame.BranchesFinished` (`/Game/Blueprint/Gameplay/BP_Character_Labyrinth.BranchesFinished` _asbp_character_labyrinth) _asbp_save_game)
  (set `/Game/Blueprint/Gameplay/System/BP_SaveGame.PathsStarted` (`/Game/Blueprint/Gameplay/BP_Character_Labyrinth.PathStarted` _asbp_character_labyrinth) _asbp_save_game)
  (set `/Game/Blueprint/Gameplay/System/BP_SaveGame.PathsFinished` (`/Game/Blueprint/Gameplay/BP_Character_Labyrinth.PathFinished` _asbp_character_labyrinth) _asbp_save_game)
  (set `/Game/Blueprint/Gameplay/System/BP_SaveGame.LevelToLoad` (`self.LevelToLoad`) _asbp_save_game)
  (set `/Game/Blueprint/Gameplay/System/BP_SaveGame.StartLocation` (`self.StartLocation`) _asbp_save_game)
  (set `/Game/Blueprint/Gameplay/System/BP_SaveGame.FogDoorStates` (`/Game/Blueprint/Gameplay/BP_Character_Labyrinth.FogDoorStates` _asbp_character_labyrinth) _asbp_save_game)
  (set `/Game/Blueprint/Gameplay/System/BP_SaveGame.SaveTime` (`KismetStringLibrary.Concat_StrStr` (`KismetStringLibrary.Conv_IntToString` _returnvalue_year) "/" (`KismetStringLibrary.Conv_IntToString` _returnvalue_month) "/" (`KismetStringLibrary.Conv_IntToString` _returnvalue_day) " " (`KismetStringLibrary.Conv_IntToString` _returnvalue_hour) ":" (`KismetStringLibrary.Conv_IntToString` _returnvalue_minute)) _asbp_save_game)
  (set `/Game/Blueprint/Gameplay/System/BP_SaveGame.PuzzlesFinished` (`/Game/Blueprint/Gameplay/BP_Character_Labyrinth.PuzzlesFinished` _asbp_character_labyrinth) _asbp_save_game)
  (`GameplayStatics.SaveGameToSlot` _asbp_save_game (`self.CurrentSaveSlotName`)))

(event `RestartLevel`
  (`GameplayStatics.DeleteGameInSlot` (`self.CurrentSaveSlotName`)))

(event `CheckSaveTime`
  (`|ExecutionSequence`
    (:`then_0`
      (bind _returnvalue (`GameplayStatics.DoesSaveGameExist` "slot1"))
      (if _returnvalue
        (bind _returnvalue_2 (`GameplayStatics.LoadGameFromSlot` "slot1"))
        (bind _asbp_save_game (cast `/Game/Blueprint/Gameplay/System/BP_SaveGame` _returnvalue_2))
        (set `self.SaveTime1` (`/Game/Blueprint/Gameplay/System/BP_SaveGame.SaveTime` _asbp_save_game))))
    (:`then_1`
      (bind _returnvalue_3 (`GameplayStatics.DoesSaveGameExist` "slot2"))
      (if _returnvalue_3
        (bind _returnvalue_4 (`GameplayStatics.LoadGameFromSlot` "slot2"))
        (bind _asbp_save_game_2 (cast `/Game/Blueprint/Gameplay/System/BP_SaveGame` _returnvalue_4))
        (set `self.SaveTime2` (`/Game/Blueprint/Gameplay/System/BP_SaveGame.SaveTime` _asbp_save_game_2))))
    (:`then_2`
      (bind _returnvalue_5 (`GameplayStatics.DoesSaveGameExist` "slot3"))
      (if _returnvalue_5
        (bind _returnvalue_6 (`GameplayStatics.LoadGameFromSlot` "slot3"))
        (bind _asbp_save_game_3 (cast `/Game/Blueprint/Gameplay/System/BP_SaveGame` _returnvalue_6))
        (set `self.SaveTime3` (`/Game/Blueprint/Gameplay/System/BP_SaveGame.SaveTime` _asbp_save_game_3))))))