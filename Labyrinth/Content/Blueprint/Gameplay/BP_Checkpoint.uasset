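; Checkpoint actor for the labyrinth that saves the game on overlap, recording the level to load and its own location as the start point.
; Hub checkpoints target the hub level and save only when it is not already set.
; Other checkpoints fire once for the player, updating the character's PathStarted or PathFinished array and building the level name from Path, Branch and Tomb.
; Both store progress through the Labyrinth game mode.
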(event `self.ReceiveActorBeginOverlap`
  (params (OtherActor :type "Actor Object Reference"))
  (bind _returnvalue (`GameplayStatics.GetPlayerPawn` 0))
  (bind _path (`self.Path`))
  (bind _tomb (`self.Tomb`))
  (bind _returnvalue_2 (`SceneComponent.K2_GetComponentLocation` (`self.DefaultSceneRoot`)))
  (bind _asbp_game_mode_labyrinth (cast `/Game/Blueprint/Gameplay/System/BP_GameMode_Labyrinth` (`GameplayStatics.GetGameMode`) :!pure true))
  (bind _asbp_game_mode_labyrinth_2 (cast `/Game/Blueprint/Gameplay/System/BP_GameMode_Labyrinth` (`GameplayStatics.GetGameMode`) :!pure true))
  (if (`self.Hub`)
    (if (!= (`/Game/Blueprint/Gameplay/System/BP_GameMode_Labyrinth.LevelToLoad` _asbp_game_mode_labyrinth) "S02_Hub")
      (set `/Game/Blueprint/Gameplay/System/BP_GameMode_Labyrinth.LevelToLoad` "S02_Hub" _asbp_game_mode_labyrinth)
      (set `/Game/Blueprint/Gameplay/System/BP_GameMode_Labyrinth.StartLocation` _returnvalue_2 _asbp_game_mode_labyrinth)
      (`/Game/Blueprint/Gameplay/System/BP_GameMode_Labyrinth.SaveGame` _asbp_game_mode_labyrinth))
    (elif (`self.HasActivated`)
      _
      (elif (== OtherActor _returnvalue)
        (bind _asbp_character_labyrinth (cast `/Game/Blueprint/Gameplay/BP_Character_Labyrinth` _returnvalue))
        (if (`self.Tomb`)
          (`KismetArrayLibrary.Array_Set` (`/Game/Blueprint/Gameplay/BP_Character_Labyrinth.PathFinished` _asbp_character_labyrinth) _path)
          (else
            (`KismetArrayLibrary.Array_Set` (`/Game/Blueprint/Gameplay/BP_Character_Labyrinth.PathStarted` _asbp_character_labyrinth) _path)))
        (set `/Game/Blueprint/Gameplay/System/BP_GameMode_Labyrinth.LevelToLoad` (`KismetStringLibrary.Conv_StringToName` (`KismetStringLibrary.Concat_StrStr` "S0" (`KismetStringLibrary.Conv_IntToString` (+ (select `int` (`self.Path`) :`0` 3 :`1` 5 :`2` 7) (select `bool` _tomb :`true` 1))) (select `int` (`self.Branch`) :`0` "A" :`1` "B" :`2` "C") (select `bool` _tomb :`false` "_Path" :`true` "_Tomb"))) _asbp_game_mode_labyrinth_2)
        (set `/Game/Blueprint/Gameplay/System/BP_GameMode_Labyrinth.StartLocation` _returnvalue_2 _asbp_game_mode_labyrinth_2)
        (`/Game/Blueprint/Gameplay/System/BP_GameMode_Labyrinth.SaveGame` _asbp_game_mode_labyrinth_2)
        (set `self.HasActivated` true)))))

(fn `UserConstructionScript`)