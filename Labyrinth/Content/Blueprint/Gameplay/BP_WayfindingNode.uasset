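; BP_WayfindingNode is an overlap checkpoint that tracks the player's movement along branches and paths in the labyrinth.
; On player overlap, it compares its OrderID with BP_Character_Labyrinth's PathProgress and calls progress or regress on the character.
; First and final node flags trigger path and branch start and end calls, with starting guarded to fire once.
; The construction script labels each node with its branch, path and order IDs.
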(event `self.ReceiveActorBeginOverlap`
  (params (OtherActor :type "Actor Object Reference"))
  (bind _returnvalue (`GameplayStatics.GetPlayerPawn` 0))
  (bind _orderid (`self.OrderID`))
  (if (== OtherActor _returnvalue)
    (bind _asbp_character_labyrinth (cast `/Game/Blueprint/Gameplay/BP_Character_Labyrinth` _returnvalue))
    (if (`self.FinalNodeOfPath`)
      (if (`self.FinalNodeOfBranch`)
        (`/Game/Blueprint/Gameplay/BP_Character_Labyrinth.EndBranch` _asbp_character_labyrinth (`self.Branch`)))
      (`/Game/Blueprint/Gameplay/BP_Character_Labyrinth.EndPath` _asbp_character_labyrinth (`self.Path`) 0))
    (bind _output (`|GetArrayItem` (`/Game/Blueprint/Gameplay/BP_Character_Labyrinth.PathProgress` _asbp_character_labyrinth) (`self.Path`)))
    (if (> _output _orderid)
      (`/Game/Blueprint/Gameplay/BP_Character_Labyrinth.RegressPath` _asbp_character_labyrinth (`self.Branch`) (`self.Path`))
      (elif (and (`self.FirstNodeOfPath`) (not (`self.HasStarted`)))
        (`/Game/Blueprint/Gameplay/BP_Character_Labyrinth.StartPath` _asbp_character_labyrinth (`self.Branch`) (`self.Path`))
        (set `self.HasStarted` true)
        (if (`self.FirstNodeOfBranch`)
          (`/Game/Blueprint/Gameplay/BP_Character_Labyrinth.StartBranch` _asbp_character_labyrinth (`self.Branch`)))
        (elif (< _output _orderid)
          (`/Game/Blueprint/Gameplay/BP_Character_Labyrinth.ProgressPath` _asbp_character_labyrinth (`self.Branch`) (`self.Path`)))))))

(fn `UserConstructionScript`
  (`TextRenderComponent.K2_SetText` (`self.ID Tag`) (`KismetTextLibrary.Conv_StringToText` (`KismetStringLibrary.Concat_StrStr` "B:" (`KismetStringLibrary.Conv_IntToString` (`self.Branch`)) " " "P:" (`KismetStringLibrary.Conv_IntToString` (`self.Path`)) " " "ID:" (`KismetStringLibrary.Conv_IntToString` (`self.OrderID`))))))