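; Player controller for the Labyrinth game that handles mouse look and the pause and settings menus.
; Look and turn axes are scaled by a sensitivity value and fed into pitch and yaw.
; Pause toggles a pause widget, game pause and cursor, but first closes any open settings widget and re-links the existing pause menu.
; It also forwards the Return action through a call and tracks whether the last key pressed came from a gamepad.
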(event `self.ReceiveBeginPlay`)

(event `InputAxis|LookUp`
  (params (AxisValue :type "Float (single-precision)"))
  (`self.AddPitchInput` (* AxisValue (`self.LookSensitivity`))))

(event `InputAxis|Turn`
  (params (AxisValue :type "Float (single-precision)"))
  (`self.AddYawInput` (* AxisValue (`self.LookSensitivity`))))

(event `TogglePause`
  (bind _pausemenuref (`self.PauseMenuRef`))
  (if (`self.PauseOpen`) :!label _label
    (if (`self.SettingsOpen`)
      (bind _foundwidgets (`WidgetBlueprintLibrary.GetAllWidgetsOfClass` "/Game/UI/UMG/Menus/W_Settings.W_Settings_C" :!label _label_2))
      (bind _output (`|GetArrayItem` _foundwidgets))
      (`/Engine/EditorBlueprintResources/StandardMacros.IsValid` _output
        (:`Is Valid`
          (`/Game/UI/UMG/Menus/W_Settings.CloseSettings` _output)
          (bind _foundwidgets_2 (`WidgetBlueprintLibrary.GetAllWidgetsOfClass` "/Game/UI/UMG/Menus/W_PauseMenu.W_PauseMenu_C"))
          (bind _output_2 (`|GetArrayItem` _foundwidgets_2))
          (`/Engine/EditorBlueprintResources/StandardMacros.IsValid` _output_2
            (:`Is Valid`
              (set `self.PauseMenuRef` _output_2)
              (set `self.SettingsOpen` false)
              (set `self.PauseOpen` true)))))
      (else
        (`/Engine/EditorBlueprintResources/StandardMacros.IsValid` _pausemenuref
          (:`Is Valid`
            (`Widget.RemoveFromParent` _pausemenuref)
            (`GameplayStatics.SetGamePaused` false)
            (set `self.bShowMouseCursor` false)
            (set `self.PauseOpen` false)))))
    (elif (`self.SettingsOpen`)
      (goto _label_2)
      (else
        (bind _returnvalue (`|CreateWidget` "/Game/UI/UMG/Menus/W_PauseMenu.W_PauseMenu_C"))
        (bind _output_get (set `self.PauseMenuRef` _returnvalue))
        (`UserWidget.AddToViewport` _output_get 0)
        (`GameplayStatics.SetGamePaused` true)
        (set `self.bShowMouseCursor` true)
        (set `self.PauseOpen` true)))))

(event `InputAction|Pause` :paused true
  (params (Key :type "Key Structure"))
  (:`Pressed`
    (goto _label)))

(event `InputAction|Return`
  (params (Key :type "Key Structure"))
  (:`Pressed`
    (`self.PressedReturn`)))

(event `Key|AnyKey` :consume false :overrideparent false
  (params (Key :type "Key Structure"))
  (:`Pressed`
    (if (`KismetInputLibrary.Key_IsGamepadKey` Key)
      (set `self.IsUsingGamepad` true)
      (else
        (set `self.IsUsingGamepad` false)))))

(fn `UserConstructionScript`)