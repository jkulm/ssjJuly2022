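; Character Blueprint for selectable musician-style characters such as Drummo and Noodler, with animation trigger flags and an erode material effect.
; Tick clears the idle, idle-to-play and soul-release flags after short delays, and construction raises the idle flag for props.
; AnimateMaterial plays a timeline driving Erode on a dynamic material created at construction.
; SetHeadSlotBlend passes a disapproval blend to the selected character's AnimBP, with the third selection unimplemented.
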(event `self.ReceiveBeginPlay`)

(event `self.ReceiveTick`
  (params (DeltaSeconds :type "Float (single-precision)"))
  (if (`self.ToIdle`)
    (`KismetSystemLibrary.Delay` 0.1)
    (set `self.ToIdle` false))
  (if (`self.ToIdleToPlay`)
    (`KismetSystemLibrary.Delay` 0.1)
    (set `self.ToIdleToPlay` false))
  (if (`self.ToSoulRelease`)
    (`KismetSystemLibrary.Delay` 0.1)
    (set `self.ToSoulRelease` false)))

(event `AnimateMaterial`
  (params (TimeDirection :type "Float (double-precision)"))
  (bind (_direction _newtrack_0) (`Timeline|Erode` :!via `PlayFromStart`)
    (:`Update`
      (`MaterialInstanceDynamic.SetScalarParameterValue` (`self.MatRef`) "Erode" _newtrack_0))))

(fn `SetHeadSlotBlend`
  (params (Blend :type "Float (double-precision)"))
  (bind _characterselection (`self.CharacterSelection`))
  (bind _returnvalue (`SkeletalMeshComponent.GetAnimInstance` (`self.SkeletalMesh`)))
  (if (== _characterselection 0)
    (bind _asabp_drummo (cast `/Game/Art/Character/Drummo/Animation/ABP_Drummo` _returnvalue))
    (set `/Game/Art/Character/Drummo/Animation/ABP_Drummo.BlendDisapprove` Blend _asabp_drummo)
    (elif (== _characterselection 1)
      (bind _asabp_noodler (cast `/Game/Art/Character/Noodler/ABP_Noodler` _returnvalue))
      (set `/Game/Art/Character/Noodler/ABP_Noodler.BlendDisapprove` Blend _asabp_noodler)
      (elif (== _characterselection 2)
        _))))

(fn `UserConstructionScript`
  (bind _skeletalmesh (`self.SkeletalMesh`))
  (bind _returnvalue (`PrimitiveComponent.CreateDynamicMaterialInstance` _skeletalmesh 0 (`PrimitiveComponent.GetMaterial` _skeletalmesh 0) "None"))
  (set `self.MatRef` _returnvalue)
  (if (`self.Prop`)
    (set `self.ToIdle` true)))