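; BP_WayfindingNode is a trigger actor that reports the player's route through branches and paths to BP_Character_Labyrinth.
; On player overlap, a final branch node calls EndBranch.
; Other nodes call RegressPath if the character's PathProgress for that path is below their OrderID, otherwise StartPath for a first node or ProgressPath.
; The construction script labels each node's IDTag with its branch, path and order ID.
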(event `self.ReceiveActorBeginOverlap`
  (params (OtherActor :type "Actor Object Reference"))
  (bind _returnvalue (`GameplayStatics.GetPlayerPawn` 0))
  (bind _path (`self.Path`))
  (bind _asbp_character_labyrinth (cast `/Game/Blueprint/Gameplay/BP_Character_Labyrinth` _returnvalue))
  (if (== OtherActor _returnvalue)
    (if (`self.FinalNodeOfBranch`)
      (`/Game/Blueprint/Gameplay/BP_Character_Labyrinth.EndBranch` _asbp_character_labyrinth (`self.Branch`))
      (elif (< (`|GetArrayItem` (`/Game/Blueprint/Gameplay/BP_Character_Labyrinth.PathProgress` _asbp_character_labyrinth) (`self.Path`)) (`self.OrderID`))
        (`/Game/Blueprint/Gameplay/BP_Character_Labyrinth.RegressPath` _asbp_character_labyrinth (`self.Branch`) (`self.Path`))
        (elif (`self.FirstNodeOfPath`)
          (`/Game/Blueprint/Gameplay/BP_Character_Labyrinth.StartPath` _asbp_character_labyrinth _path _path)
          (`/Game/Blueprint/Gameplay/BP_Character_Labyrinth.StartPath` _asbp_character_labyrinth _path _path)
          (else
            (`/Game/Blueprint/Gameplay/BP_Character_Labyrinth.ProgressPath` _asbp_character_labyrinth _path 0)))))))

(fn `UserConstructionScript`
  (`TextRenderComponent.K2_SetText` (`self.ID Tag`) (`KismetTextLibrary.Conv_StringToText` (`KismetStringLibrary.Concat_StrStr` "B:" (`KismetStringLibrary.Conv_IntToString` (`self.Branch`)) " " "P:" (`KismetStringLibrary.Conv_IntToString` (`self.Path`)) " " "ID:" (`KismetStringLibrary.Conv_IntToString` (`self.OrderID`))))))