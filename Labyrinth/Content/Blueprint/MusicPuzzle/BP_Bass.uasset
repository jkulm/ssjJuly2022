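; BP_Bass is a six-string bass for the music puzzle, or a playable prop when Prop is set.
; Grabbing a string collider plays its note at that location, spikes its animation value and, unless a prop, reports the index to BP_PuzzleManager.
; Tick decays those values per frame into a dynamic string material.
; Separate events activate per-string Niagara effects, set their duration and recolor the strings.
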(event `self.ReceiveBeginPlay`
  (if (not (`self.Prop`))
    (bind _outactors (`GameplayStatics.GetAllActorsOfClass` "/Game/Blueprint/MusicPuzzle/BP_PuzzleManager.BP_PuzzleManager_C" :!label _label))
    (bind _output (`|GetArrayItem` _outactors))
    (`/Engine/EditorBlueprintResources/StandardMacros.IsValid` _output
      (:`Is Valid`
        (set `self.PuzzleManagerRef` _output))
      (:`Is Not Valid`
        (goto _label)))))

(event `self.ReceiveTick`
  (params (DeltaSeconds :type "Float (single-precision)"))
  (bind _stringanimdecay (`self.StringAnimDecay`))
  ;[1 1 1] Decay Animation Values
  (`|ExecutionSequence`
    (:`then_0`
      (bind _outvalue (`self.AnimDecay` (`self.String1Animation`) _stringanimdecay))
      (bind _output_get (set `self.String1Animation` _outvalue))
      (`MaterialInstanceDynamic.SetScalarParameterValue` (`self.StringMat`) "BP_Value1" _output_get))
    (:`then_1`
      (bind _outvalue_2 (`self.AnimDecay` (`self.String2Animation`) _stringanimdecay))
      (bind _output_get_2 (set `self.String2Animation` _outvalue_2))
      (`MaterialInstanceDynamic.SetScalarParameterValue` (`self.StringMat`) "BP_Value2" _output_get_2))
    (:`then_2`
      (bind _outvalue_3 (`self.AnimDecay` (`self.String3Animation`) _stringanimdecay))
      (bind _output_get_3 (set `self.String3Animation` _outvalue_3))
      (`MaterialInstanceDynamic.SetScalarParameterValue` (`self.StringMat`) "BP_Value3" _output_get_3))
    (:`then_3`
      (bind _outvalue_4 (`self.AnimDecay` (`self.String4Animation`) _stringanimdecay))
      (bind _output_get_4 (set `self.String4Animation` _outvalue_4))
      (`MaterialInstanceDynamic.SetScalarParameterValue` (`self.StringMat`) "BP_Value4" _output_get_4))
    (:`then_4`
      (bind _outvalue_5 (`self.AnimDecay` (`self.String5Animation`) _stringanimdecay))
      (bind _output_get_5 (set `self.String5Animation` _outvalue_5))
      (`MaterialInstanceDynamic.SetScalarParameterValue` (`self.StringMat`) "BP_Value5" _output_get_5))
    (:`then_5`
      (bind _outvalue_6 (`self.AnimDecay` (`self.String6Animation`) _stringanimdecay))
      (bind _output_get_6 (set `self.String6Animation` _outvalue_6))
      (`MaterialInstanceDynamic.SetScalarParameterValue` (`self.StringMat`) "BP_Value6" _output_get_6))))

(event `/Game/Blueprint/Interfaces/BPI_Grab.GrabObject`
  (params (HitCollider :type "PrimitiveComponent Object Reference"))
  (bind _stringcolliders (`self.StringColliders`))
  (bind _returnvalue (`KismetArrayLibrary.Array_Find` _stringcolliders HitCollider))
  (if (`KismetArrayLibrary.Array_Contains` _stringcolliders HitCollider)
    (`|ExecutionSequence`
      (:`then_0`
        (if (== _returnvalue 0)
          (set `self.String1Animation` 1.0)
          (`FMODBlueprintStatics.PlayEventAtLocation` (`|GetArrayItem` (`self.NoteList`) _returnvalue) (`KismetMathLibrary.MakeTransform` (`SceneComponent.K2_GetComponentLocation` (`|GetArrayItem` (`self.StringColliders`) _returnvalue))) :!label _label_2)
          (if (not (`self.Prop`))
            (`/Game/Blueprint/MusicPuzzle/BP_PuzzleManager.PlayerInput` (`self.PuzzleManagerRef`) _returnvalue null self))))
      (:`then_1`
        (if (== _returnvalue 1)
          (set `self.String2Animation` 1.0)
          (goto _label_2)))
      (:`then_2`
        (if (== _returnvalue 2)
          (set `self.String3Animation` 1.0)
          (goto _label_2)))
      (:`then_3`
        (if (== _returnvalue 3)
          (set `self.String4Animation` 1.0)
          (goto _label_2)))
      (:`then_4`
        (if (== _returnvalue 4)
          (set `self.String5Animation` 1.0)
          (goto _label_2)))
      (:`then_5`
        (if (== 5 _returnvalue)
          (set `self.String6Animation` 1.0)
          (goto _label_2))))))

(event `TriggerString`
  (params (Note :type Integer))
  (`ActorComponent.Activate` (select `int` Note :`0` (`self.Niagara`) :`1` (`self.Niagara1`) :`2` (`self.Niagara2`) :`3` (`self.Niagara3`) :`4` (`self.Niagara4`) :`5` (`self.Niagara5`)) true))

(event `SetStringDefaults`
  (params (Duration :type "Float (double-precision)"))
  (for _array_element (`self.NiagaraSystems`)
    (`FXSystemComponent.SetFloatParameter` _array_element "User.Duration" Duration)))

(event `SetColor`
  (params (NewParam :type "LinearColor Structure"))
  (`MaterialInstanceDynamic.SetVectorParameterValue` (`self.StringMat`) "BP_Color" NewParam))

(fn `AnimDecay`
  (params (InValue :type "Float (double-precision)") (DecayRate :type "Float (double-precision)"))
  (returns (OutValue :type "Float (double-precision)"))
  (if (> InValue 0.0)
    (return (- InValue (/ 1.0 DecayRate)))))

(fn `UserConstructionScript`
  (bind _niagarasystems (`self.NiagaraSystems`))
  (bind _mesh (`self.Mesh`))
  (bind _stringcolliders (`self.StringColliders`))
  (bind _returnvalue (`PrimitiveComponent.CreateDynamicMaterialInstance` _mesh 2 (`PrimitiveComponent.GetMaterial` _mesh 2) "None"))
  (set `self.StringMat` _returnvalue)
  (`|ExecutionSequence`
    (:`then_0`
      (`KismetArrayLibrary.Array_Clear` _stringcolliders)
      (`KismetArrayLibrary.Array_Add` _stringcolliders (`self.String1`))
      (`KismetArrayLibrary.Array_Add` _stringcolliders (`self.String2`))
      (`KismetArrayLibrary.Array_Add` _stringcolliders (`self.String3`))
      (`KismetArrayLibrary.Array_Add` _stringcolliders (`self.String4`))
      (`KismetArrayLibrary.Array_Add` _stringcolliders (`self.String5`))
      (`KismetArrayLibrary.Array_Add` _stringcolliders (`self.String6`)))
    (:`then_1`
      (`KismetArrayLibrary.Array_Clear` _niagarasystems)
      (`KismetArrayLibrary.Array_Add` _niagarasystems (`self.Niagara`))
      (`KismetArrayLibrary.Array_Add` _niagarasystems (`self.Niagara1`))
      (`KismetArrayLibrary.Array_Add` _niagarasystems (`self.Niagara2`))
      (`KismetArrayLibrary.Array_Add` _niagarasystems (`self.Niagara3`))
      (`KismetArrayLibrary.Array_Add` _niagarasystems (`self.Niagara4`))
      (`KismetArrayLibrary.Array_Add` _niagarasystems (`self.Niagara5`)))))