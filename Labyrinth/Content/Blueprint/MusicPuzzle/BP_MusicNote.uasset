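; BP_MusicNote is a timed note actor in the music puzzle, shown as an instrument-specific Niagara effect for drum, bass or flute.
; BeginPlay spawns the inactive effect, and SetData stores the note data, sets its radius and duration, and activates it.
; Parallel delays open the input window around the lead time and, at its end, report a miss to the PuzzleManager.
; DestroyMusicNote removes the manager's first NoteList entry and destroys the actor.
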(event `self.ReceiveBeginPlay`
  (bind _returnvalue (`NiagaraFunctionLibrary.SpawnSystemAttached` (`|GetArrayItem` (`self.NiagaraSystems`) (select `/Game/Data/ENUM_Instruments` (`self.Instrument`) :`NewEnumerator1` 1 :`NewEnumerator2` 2)) (`self.DefaultSceneRoot`) "None" (0.0 0.0 0.0) (struct) "SnapToTargetIncludingScale" true false))
  (set `self.NiagaraSystem` _returnvalue))

(event `SetData`
  (params (Instrument :type "/Game/Data/ENUM_Instruments Enum" :default "NewEnumerator0") (LeadTime :type "Float (double-precision)") (InputWindow :type "Float (double-precision)") (ScaleFactor :type "Float (double-precision)") (Note :type Integer) (PuzzleManager :type "/Game/Blueprint/MusicPuzzle/BP_PuzzleManager Object Reference"))
  (set `self.Instrument` Instrument)
  (set `self.LeadTime` LeadTime)
  (set `self.InputWindow` InputWindow)
  (set `self.ScaleFactor` ScaleFactor)
  (set `self.Note` Note)
  (set `self.PuzzleManager` PuzzleManager)
  (`self.StartSystem`))

(event `StartSystem`
  (bind _niagarasystem (`self.NiagaraSystem`))
  (`FXSystemComponent.SetFloatParameter` _niagarasystem "User.Radius" (`self.ScaleFactor`))
  (`FXSystemComponent.SetFloatParameter` _niagarasystem "User.Duration" (+ (`self.LeadTime`) (* (`self.InputWindow`) 0.5)))
  (`ActorComponent.Activate` _niagarasystem true)
  (`self.TriggerInputWindow`)
  (`self.DetectMiss`))

(event `TriggerInputWindow`
  (`KismetSystemLibrary.Delay` (- (`self.LeadTime`) (* (`self.InputWindow`) 0.5)))
  (set `self.IsInputValid` true))

(event `DetectMiss`
  (`KismetSystemLibrary.Delay` (+ (`self.LeadTime`) (* (`self.InputWindow`) 0.5)))
  (`/Game/Blueprint/MusicPuzzle/BP_PuzzleManager.TrackFailure` (`self.PuzzleManager`))
  (`self.DestroyMusicNote`))

(event `DestroyMusicNote`
  (`KismetArrayLibrary.Array_Remove` (`/Game/Blueprint/MusicPuzzle/BP_PuzzleManager.NoteList` (`self.PuzzleManager`)))
  (`self.K2_DestroyActor`))

(fn `UserConstructionScript`)