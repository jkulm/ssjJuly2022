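; Interactive drum for the music puzzle that plays its selected note when grabbed and reports the hit to BP_PuzzleManager.
; Drums flagged as Prop skip the manager; others look it up on BeginPlay, retrying in an unbounded loop until valid.
; A dynamic material on the drum head shows a hit pulse that decays each Tick.
; SetColor tints the head green or red for feedback, or black on reset.
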(event `self.ReceiveBeginPlay`
  (if (not (`self.Prop`))
    (bind _outactors (`GameplayStatics.GetAllActorsOfClass` "/Game/Blueprint/MusicPuzzle/BP_PuzzleManager.BP_PuzzleManager_C" :!label _label))
    (bind _output (`|GetArrayItem` _outactors))
    (`/Engine/EditorBlueprintResources/StandardMacros.IsValid` _output
      (:`Is Valid`
        (set `self.PuzzleManagerRef` _output))
      (:`Is Not Valid`
        (goto _label)))))

(event `self.ReceiveTick`
  (params (DeltaSeconds :type "Float (single-precision)"))
  (bind _drumanimation (`self.DrumAnimation`))
  (if (> _drumanimation 0.0)
    (bind _output_get (set `self.DrumAnimation` (- _drumanimation (/ 1.0 (`self.DrumHeadDecay`)))))
    (`MaterialInstanceDynamic.SetScalarParameterValue` (`self.DrumHeadMat`) "BP_Value" _output_get)))

(event `/Game/Blueprint/Interfaces/BPI_Grab.GrabObject`
  (params (HitCollider :type "PrimitiveComponent Object Reference"))
  (`FMODBlueprintStatics.PlayEventAtLocation` (`|GetArrayItem` (`self.NoteList`) (`self.NoteSelection`)) (`KismetMathLibrary.MakeTransform` (`SceneComponent.K2_GetComponentLocation` (`self.SpawnLocationObject`))))
  (set `self.DrumAnimation` 1.0)
  (if (not (`self.Prop`))
    (`/Game/Blueprint/MusicPuzzle/BP_PuzzleManager.PlayerInput` (`self.PuzzleManagerRef`) (`self.NoteSelection`) self null)))

(event `/Game/Blueprint/Interfaces/BPI_Grab.ReleaseObject`)

(event `Set Color`
  (params (Good :type Boolean) (Reset :type Boolean))
  (bind _drumheadmat (`self.DrumHeadMat`))
  (if Reset
    (`MaterialInstanceDynamic.SetVectorParameterValue` (`self.DrumHeadMat`) "BP_Color" (struct :`A` 1.0))
    (elif Good
      (`MaterialInstanceDynamic.SetVectorParameterValue` _drumheadmat "BP_Color" (struct :`G` 1.0 :`A` 1.0))
      (else
        (`MaterialInstanceDynamic.SetVectorParameterValue` _drumheadmat "BP_Color" (struct :`R` 1.0 :`A` 1.0))))))

(fn `UserConstructionScript`
  (bind _mesh (`self.Mesh`))
  (bind _returnvalue (`PrimitiveComponent.CreateDynamicMaterialInstance` _mesh 2 (`PrimitiveComponent.GetMaterial` _mesh 2) "None"))
  (set `self.DrumHeadMat` _returnvalue)
  (`SceneComponent.SetRelativeScale3D` _mesh (`self.MeshScale`))
  (set `self.SpawnLocation` (`SceneComponent.K2_GetComponentLocation` (`self.SpawnLocationObject`))))